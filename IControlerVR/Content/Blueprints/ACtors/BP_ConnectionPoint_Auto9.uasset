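; BP_ConnectionPoint_Auto9 is a connection beam between two BP_Activity actors that the player can delete by hand.
; A particle beam with a configurable color takes its endpoints from SetBeamSource and SetBeamTarget, which also shows the Cube handle.
; The Cube changes material while a BP_Hand overlaps it, and Tick polls that hand's trigger.
; A trigger press calls RemoveBeam, which removes the target from the source's Targets and destroys the actor.
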(event `self.ReceiveBeginPlay`
  ;[1 1 1] Begin Play
  (`ParticleSystemComponent.SetActorParameter` (`self.Beam`) "BeamTarget" self)
  (bind _asbp_player_pawn (cast `/Game/Blueprints/Pawns/BP_PlayerPawn` (`GameplayStatics.GetPlayerPawn` 0)))
  (add `/Game/Blueprints/Pawns/BP_PlayerPawn.OnTriggerPressed` _asbp_player_pawn (delegate `OnTriggerPressed_Event_1`)))

(event `OnTriggerPressed_Event_1`
  ;[1 1 1] Begin Play
)

(event `self.ReceiveTick`
  (params (DeltaSeconds :type "Float (single-precision)"))
  ;[1 1 1] Tick Event
  (if (`self.IsBeamOverlap`)
    (if (`/Game/Blueprints/Actors/BP_Hand.TriggerPressed` (`self.OverlappingHAnd`))
      (`self.RemoveBeam`))))

(event `self.Cube.OnComponentBeginOverlap`
  (params (OverlappedComponent :type "PrimitiveComponent Object Reference") (OtherActor :type "Actor Object Reference") (OtherComp :type "PrimitiveComponent Object Reference") (OtherBodyIndex :type Integer) (bFromSweep :type Boolean) (SweepResult :type "HitResult Structure (by ref)"))
  ;[1 1 1] Cube Begin Overlap
  (bind _asbp_hand (cast `/Game/Blueprints/Actors/BP_Hand` OtherActor))
  (set `self.OverlappingHAnd` _asbp_hand)
  (`PrimitiveComponent.SetMaterial` (`self.Cube`) 0 "/Game/Materials/Transparant.Transparant")
  (set `self.IsBeamOverlap` true)
  (if (`/Game/Blueprints/Actors/BP_Hand.TriggerPressed` _asbp_hand)
    (`PrimitiveComponent.SetMaterial` (`self.Cube`) 0 "/Game/StarterContent/Materials/M_Glass.M_Glass")
    (`self.RemoveBeam`)))

(event `self.Cube.OnComponentEndOverlap`
  (params (OverlappedComponent :type "PrimitiveComponent Object Reference") (OtherActor :type "Actor Object Reference") (OtherComp :type "PrimitiveComponent Object Reference") (OtherBodyIndex :type Integer))
  ;[1 1 1] Cube End Overlap
  (cast `/Game/Blueprints/Actors/BP_Hand` OtherActor)
  (`PrimitiveComponent.SetMaterial` (`self.Cube`) 0 "/Game/Materials/Red.Red")
  (set `self.IsBeamOverlap` false))

(fn `HasSource`
  (returns (HasSource :type Boolean))
  (`/Engine/EditorBlueprintResources/StandardMacros.IsValid` (`self.Source`)
    (:`Is Valid`
      (return true))
    (:`Is Not Valid`
      (return false))))

(fn `RemoveBeam`
  (bind _asbp_activity (cast `/Game/Blueprints/ACtors/Activities/BP_Activity` (`self.Source`)))
  (bind _asbp_activity_2 (cast `/Game/Blueprints/ACtors/Activities/BP_Activity` (`self.Target`)))
  (bind _targets (`/Game/Blueprints/ACtors/Activities/BP_Activity.Targets` _asbp_activity))
  (if (`KismetArrayLibrary.Array_Contains` _targets _asbp_activity_2)
    (`KismetArrayLibrary.Array_RemoveItem` _targets _asbp_activity_2)
    (`self.K2_DestroyActor`)))

(fn `SetBeamSource`
  (params (Source :type "Actor Object Reference"))
  (bind _output_get (set `self.Source` Source))
  (`ParticleSystemComponent.SetActorParameter` (`self.Beam`) "BeamSource" _output_get))

(fn `SetBeamTarget`
  (params (Target :type "Actor Object Reference"))
  (bind _output_get (set `self.Target` Target))
  (`ParticleSystemComponent.SetActorParameter` (`self.Beam`) "BeamTarget" _output_get)
  (`SceneComponent.SetVisibility` (`self.Cube`) true true))

(fn `UserConstructionScript`
  (set `self.BeamEmitter` (`self.Beam`))
  (bind _returnvalue (`PrimitiveComponent.CreateDynamicMaterialInstance` (`self.Beam`) 0 "/Game/Materials/Beam.Beam"))
  (`MaterialInstanceDynamic.SetVectorParameterValue` _returnvalue "BeamColor" (`self.BeamColor`))
  (`PrimitiveComponent.SetMaterial` (`self.Beam`) 0 _returnvalue))