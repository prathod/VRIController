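; BP_BPMLane is a lane actor that labels itself and marks a relative spawn point, apparently for placing the next lane.
; The construction script writes RolLane's Rol value into its TextRender.
; GetRelativeSpawnPoint returns the relative location of the NextLane component.
; The event graph has no active runtime logic.
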(event `self.ReceiveBeginPlay`)

(fn `GetRelativeSpawnPoint`
  (returns (GetRelative :type "Vector Structure"))
  (return (`SceneComponent.RelativeLocation` (`self.NextLane`))))

(fn `UserConstructionScript`
  (`TextRenderComponent.K2_SetText` (`self.TextRender`) (`KismetTextLibrary.Conv_StringToText` (`/Game/Blueprints/ACtors/BP_Rol.Rol` (`self.RolLane`)))))