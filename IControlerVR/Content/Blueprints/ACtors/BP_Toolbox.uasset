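; BP_Toolbox is a toolbox actor that spawns BP_Activity or BP_Decision actors when a BP_Hand overlaps the matching button component.
; Activities spawn slightly in front of their button and decisions at theirs, both only under authority.
; A single IsCreated flag blocks further spawns of either type until an activity leaves Cube1 or a decision leaves DecisionButton.
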(event `self.Cube1.OnComponentEndOverlap`
  (params (OverlappedComponent :type "PrimitiveComponent Object Reference") (OtherActor :type "Actor Object Reference") (OtherComp :type "PrimitiveComponent Object Reference") (OtherBodyIndex :type Integer))
  ;[1 1 1] Activity Overlap
  (cast `/Game/Blueprints/ACtors/Activities/BP_Activity` OtherActor)
  (set `self.IsCreated` false))

(event `self.ActivityButton.OnComponentBeginOverlap`
  (params (OverlappedComponent :type "PrimitiveComponent Object Reference") (OtherActor :type "Actor Object Reference") (OtherComp :type "PrimitiveComponent Object Reference") (OtherBodyIndex :type Integer) (bFromSweep :type Boolean) (SweepResult :type "HitResult Structure (by ref)"))
  (bind _activitybutton (`self.ActivityButton`))
  (bind (_returnvalue_location _returnvalue_rotation) (`KismetMathLibrary.BreakTransform` (`SceneComponent.K2_GetComponentToWorld` _activitybutton)))
  ;[1 1 1] Activity Overlap
  (cast `/Game/Blueprints/Actors/BP_Hand` OtherActor)
  (if (not (`self.IsCreated`))
    (`KismetSystemLibrary.PrintString` "Hello")
    (`self.SpawnActivity` (+ _returnvalue_location (* (`SceneComponent.GetForwardVector` _activitybutton) 3)) _returnvalue_rotation)
    (set `self.IsCreated` true)))

(event `SpawnActivity`
  (params (Location :type "Vector Structure") (Rotation :type "Rotator Structure"))
  (`/Engine/EditorBlueprintResources/ActorMacros.Switch Has Authority`
    (:`Authority`
      (`|SpawnActorFromClass` "/Game/Blueprints/ACtors/Activities/BP_Activity.BP_Activity_C" (`KismetMathLibrary.MakeTransform` Location Rotation (1.0 1.0 1.0)) "AdjustIfPossibleButAlwaysSpawn" "OverrideRootScale"))))

(event `self.DecisionButton.OnComponentBeginOverlap`
  (params (OverlappedComponent :type "PrimitiveComponent Object Reference") (OtherActor :type "Actor Object Reference") (OtherComp :type "PrimitiveComponent Object Reference") (OtherBodyIndex :type Integer) (bFromSweep :type Boolean) (SweepResult :type "HitResult Structure (by ref)"))
  (bind (_returnvalue_location _returnvalue_rotation) (`KismetMathLibrary.BreakTransform` (`SceneComponent.K2_GetComponentToWorld` (`self.DecisionButton`))))
  (cast `/Game/Blueprints/Actors/BP_Hand` OtherActor)
  (if (not (`self.IsCreated`))
    (`self.SpawnDecision` _returnvalue_location _returnvalue_rotation)
    (set `self.IsCreated` true)))

(event `SpawnDecision`
  (params (Location :type "Vector Structure") (Rotation :type "Rotator Structure"))
  (`/Engine/EditorBlueprintResources/ActorMacros.Switch Has Authority`
    (:`Authority`
      (`|SpawnActorFromClass` "/Game/Blueprints/ACtors/Activities/BP_Decision.BP_Decision_C" (`KismetMathLibrary.MakeTransform` Location Rotation) "AdjustIfPossibleButAlwaysSpawn" "OverrideRootScale"))))

(event `self.DecisionButton.OnComponentEndOverlap`
  (params (OverlappedComponent :type "PrimitiveComponent Object Reference") (OtherActor :type "Actor Object Reference") (OtherComp :type "PrimitiveComponent Object Reference") (OtherBodyIndex :type Integer))
  (cast `/Game/Blueprints/ACtors/Activities/BP_Decision` OtherActor)
  (set `self.IsCreated` false))

(fn `UserConstructionScript`)