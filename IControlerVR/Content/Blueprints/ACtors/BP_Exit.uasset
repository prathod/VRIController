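; BP_Exit is a host-only exit trigger that sends the session to the Department map via ServerTravel as a listen server.
; It destroys itself on remote instances at BeginPlay.
; A BP_Hand overlapping the cube turns it green and starts a looping one-second countdown shown on a text render, travelling when it reaches zero.
; Ending the overlap clears the timer, resets the countdown and label, and turns the cube red.
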(event `self.ReceiveBeginPlay`
  (`/Engine/EditorBlueprintResources/ActorMacros.Switch Has Authority`
    (:`Remote`
      (`self.K2_DestroyActor`))))

(event `self.Cube.OnComponentBeginOverlap`
  (params (OverlappedComponent :type "PrimitiveComponent Object Reference") (OtherActor :type "Actor Object Reference") (OtherComp :type "PrimitiveComponent Object Reference") (OtherBodyIndex :type Integer) (bFromSweep :type Boolean) (SweepResult :type "HitResult Structure (by ref)"))
  (`/Engine/EditorBlueprintResources/ActorMacros.Switch Has Authority`
    (:`Authority`
      (cast `/Game/Blueprints/Actors/BP_Hand` OtherActor)
      (`self.UpdateTimer`)
      (bind _returnvalue (`KismetSystemLibrary.K2_SetTimer` null "UpdateTimer" 1.0 true))
      (set `self.TimeHandler` _returnvalue)
      (`PrimitiveComponent.SetMaterial` (`self.Cube`) 0 "/Game/Materials/Green.Green"))))

(event `self.Cube.OnComponentEndOverlap`
  (params (OverlappedComponent :type "PrimitiveComponent Object Reference") (OtherActor :type "Actor Object Reference") (OtherComp :type "PrimitiveComponent Object Reference") (OtherBodyIndex :type Integer))
  (`/Engine/EditorBlueprintResources/ActorMacros.Switch Has Authority`
    (:`Authority`
      (cast `/Game/Blueprints/Actors/BP_Hand` OtherActor)
      (`self.ResetTimer`)
      (`PrimitiveComponent.SetMaterial` (`self.Cube`) 0 "/Game/Materials/Red.Red"))))

(event `GoToDepartments`
  (`KismetSystemLibrary.ExecuteConsoleCommand` "ServerTravel Department?listen"))

(fn `ResetTimer`
  (set `self.Time` 4)
  (`KismetSystemLibrary.K2_ClearAndInvalidateTimerHandle` (`self.TimeHandler`))
  (`TextRenderComponent.K2_SetText` (`self.TextRender`) (`KismetTextLibrary.Conv_StringToText` "Exit to department overview")))

(fn `UpdateTimer`
  (bind _output_get (set `self.Time` (- (`self.Time`) 1)))
  (`TextRenderComponent.K2_SetText` (`self.TextRender`) (`KismetTextLibrary.Conv_StringToText` (`KismetStringLibrary.Concat_StrStr` "Exit in: " (`KismetStringLibrary.Conv_IntToString` _output_get))))
  (if (<= (`self.Time`) 0)
    (`self.GoToDepartments`)))

(fn `UserConstructionScript`)