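; Player hand actor that moves Activity actors and draws connection patterns between them.
; Controller overlaps track the current IActivity, which grabbing attaches to the hand until released.
; Drawing stores the first activity, shows a beam from it to the hand, then calls ConnectActivity on later targets, cancelling on failure or empty space.
; Attach, detach and pattern requests execute only with authority; a material swap highlights the hand.
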(event `AttachActivity`
  (params (`Target activity` :type "/Game/Blueprints/ACtors/Activities/BP_Activity Object Reference"))
  ;[1 1 1] Start moving a activity
  (`self.K2_AttachToActor` `Target activity` self "None" "KeepWorld" "KeepWorld" "KeepWorld" true)
  (set `self.MovingActor` `Target activity`))

(event `ShowPreview`
  (params (Activity :type "/Game/Blueprints/ACtors/Activities/BP_Activity Object Reference"))
  ;[1 1 1] Show preview of connecting
  (bind _returnvalue (`|SpawnActorFromClass` "/Game/Blueprints/ACtors/BP_ConnectionPoint_Auto9.BP_ConnectionPoint_C" (`KismetMathLibrary.MakeTransform` (0.0 0.0 0.0)) "Undefined" "OverrideRootScale" null (struct :`R` 0.65)))
  (bind _output_get (set `self.ConnectingParticle` _returnvalue))
  (`/Game/Blueprints/ACtors/BP_ConnectionPoint_Auto9.SetBeamSource` _output_get Activity)
  (`/Game/Blueprints/ACtors/BP_ConnectionPoint_Auto9.SetBeamTarget` _output_get self))

(event `RequestAttachment`
  (params (`Target activity` :type "/Game/Blueprints/ACtors/Activities/BP_Activity Object Reference"))
  ;[1 1 1] Start moving a activity
  (`/Engine/EditorBlueprintResources/ActorMacros.Switch Has Authority`
    (:`Authority`
      (`self.AttachActivity` `Target activity`))))

(event `StartMovingActivity`
  (bind _overlappingactivity (`self.OverlappingActivity`))
  ;[1 1 1] Start moving a activity
  (`/Engine/EditorBlueprintResources/StandardMacros.IsValid` (`KismetSystemLibrary.Conv_InterfaceToObject` _overlappingactivity)
    (:`Is Valid`
      (bind _asbp_activity (cast `/Game/Blueprints/ACtors/Activities/BP_Activity` _overlappingactivity))
      (`self.RequestAttachment` _asbp_activity))))

(event `self.ReceiveBeginPlay`
  (bind _returnvalue (`GameplayStatics.GetPlayerController` 0))
  ;[1 1 1] Set references
  (cast `/Game/Blueprints/PlayerControllers/BP_PlayerController` _returnvalue)
  (bind _asbp_player_pawn (cast `/Game/Blueprints/Pawns/BP_PlayerPawn` (`Controller.K2_GetPawn` _returnvalue)))
  (set `self.PlayerPawn` _asbp_player_pawn))

(event `DisablePreview`
  (bind _connectingparticle (`self.ConnectingParticle`))
  ;[1 1 1] Destroy the preview of connecting
  (`/Engine/EditorBlueprintResources/StandardMacros.IsValid` _connectingparticle
    (:`Is Valid`
      (`self.K2_DestroyActor` _connectingparticle))))

(event `StopMovingActivity`
  ;[1 1 1] Stop moving a activity
  (`/Engine/EditorBlueprintResources/StandardMacros.IsValid` (`self.MovingActor`)
    (:`Is Valid`
      (`self.RequestDettach`))))

(event `StartDrawingPatern`
  ;[1 1 1] Start drawing the patern
  (`/Engine/EditorBlueprintResources/StandardMacros.IsValid` (`KismetSystemLibrary.Conv_InterfaceToObject` (`self.OverlappingActivity`))
    (:`Is Valid`
      (bind _asbp_activity (cast `/Game/Blueprints/ACtors/Activities/BP_Activity` (`self.OverlappingActivity`)))
      (`self.SendDrawPaternRequest` _asbp_activity))
    (:`Is Not Valid`
      (`self.StopDrawingRequest`))))

(event `SendDrawPaternRequest`
  (params (ConnectingActor :type "/Game/Blueprints/ACtors/Activities/BP_Activity Object Reference"))
  ;[1 1 1] Try to start drawing on the server
  (`/Engine/EditorBlueprintResources/ActorMacros.Switch Has Authority`
    (:`Authority`
      (`self.CreatePatern` ConnectingActor))))

(event `RequestDettach`
  ;[1 1 1] Stop moving a activity
  (`/Engine/EditorBlueprintResources/ActorMacros.Switch Has Authority`
    (:`Authority`
      (`self.DettachActivity`))))

(event `DettachActivity`
  ;[1 1 1] Stop moving a activity
  (`self.K2_DetachFromActor` (`self.MovingActor`) "KeepWorld" "KeepWorld" "KeepWorld"))

(event `StopDrawingRequest`
  ;[1 1 1] Stop drawing on the server
  (`/Engine/EditorBlueprintResources/ActorMacros.Switch Has Authority`
    (:`Authority`
      (`self.StopconnectingPatern`))))

(event `self.Controller.OnComponentBeginOverlap`
  (params (OverlappedComponent :type "PrimitiveComponent Object Reference") (OtherActor :type "Actor Object Reference") (OtherComp :type "PrimitiveComponent Object Reference") (OtherBodyIndex :type Integer) (bFromSweep :type Boolean) (SweepResult :type "HitResult Structure (by ref)"))
  ;[1 1 1] On overlap events
  (bind _asiactivity (cast `/Game/Blueprints/Interfaces/IActivity` OtherActor))
  (set `self.OverlappingActivity` _asiactivity))

(event `self.Controller.OnComponentEndOverlap`
  (params (OverlappedComponent :type "PrimitiveComponent Object Reference") (OtherActor :type "Actor Object Reference") (OtherComp :type "PrimitiveComponent Object Reference") (OtherBodyIndex :type Integer))
  ;[1 1 1] On overlap events
  (cast `/Game/Blueprints/Interfaces/IActivity` OtherActor)
  (set `self.OverlappingActivity` null))

(fn `ConnectingPatern`
  (params (Target :type "/Game/Blueprints/ACtors/Activities/BP_Activity Object Reference"))
  ;[1 1 1] Connect the activitys if there is a old one
  (`/Engine/EditorBlueprintResources/StandardMacros.IsValid` (`self.OldActivity`)
    (:`Is Valid`
      (bind _alreadyconnected (`/Game/Blueprints/ACtors/Activities/BP_Activity.ConnectActivity` (`self.OldActivity`) Target))
      (if (not _alreadyconnected)
        (`self.StopconnectingPatern`)))
    (:`Is Not Valid`
      (set `self.OldActivity` Target))))

(fn `CreatePatern`
  (params (ConnectingActor :type "/Game/Blueprints/ACtors/Activities/BP_Activity Object Reference"))
  (`/Engine/EditorBlueprintResources/StandardMacros.IsValid` (`self.ConnectingParticle`)
    (:`Is Valid`
      _)
    (:`Is Not Valid`
      (`self.ShowPreview` ConnectingActor)))
  (`self.ConnectingPatern` ConnectingActor))

(fn `HighlightHand`
  (params (IsHighlighting :type Boolean))
  (bind _controller (`self.Controller`))
  (if IsHighlighting
    (`PrimitiveComponent.SetMaterial` _controller 0 "/Game/StarterContent/Props/Materials/M_Door.M_Door")
    (else
      (`PrimitiveComponent.SetMaterial` _controller 0 "/Game/Materials/LightBlue.LightBlue"))))

(fn `StopconnectingPatern`
  (set `self.OldActivity` null)
  ;[1 1 1] Remove the preview
  (`self.DisablePreview`))

(fn `UserConstructionScript`)