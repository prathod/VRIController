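; BP_Menu is a VR session menu actor with Host and Join buttons that respond to hand overlaps.
; Overlapping either button with a BP_Hand highlights the hand and sets a shared EnableTrigger flag, both cleared when the overlap ends.
; The player controller's trigger event, bound on BeginPlay, calls HostSession on BP_GameInstance while enabled.
; Both buttons currently lead to hosting, as no join call exists.
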(event `self.ReceiveBeginPlay`
  (bind _asbp_player_controller (cast `/Game/Blueprints/PlayerControllers/BP_PlayerController` (`GameplayStatics.GetPlayerController` 0)))
  (bind _output_get (set `self.BP_PlayerController` _asbp_player_controller))
  (add `/Game/Blueprints/PlayerControllers/BP_PlayerController.OnTriggerPressed` _output_get (delegate `TriggerPressed`)))

(event `TriggerPressed`
  (params (IsLeft :type Boolean))
  (if (`self.EnableTrigger`)
    (bind _asbp_game_instance (cast `/Game/Blueprints/GameInstances/BP_GameInstance` (`GameplayStatics.GetGameInstance`)))
    (`/Game/Blueprints/GameInstances/BP_GameInstance.HostSession` _asbp_game_instance true)))

(event `self.HostButton.OnComponentBeginOverlap`
  (params (OverlappedComponent :type "PrimitiveComponent Object Reference") (OtherActor :type "Actor Object Reference") (OtherComp :type "PrimitiveComponent Object Reference") (OtherBodyIndex :type Integer) (bFromSweep :type Boolean) (SweepResult :type "HitResult Structure (by ref)"))
  ;[1 1 1] Highlight Controller on Overlap
  (bind _asbp_hand (cast `/Game/Blueprints/Actors/BP_Hand` OtherActor))
  (`/Game/Blueprints/Actors/BP_Hand.HighlightHand` (stale `self.JoinButton.OnComponentBeginOverlap` _asbp_hand) true :!label _label)
  (`/Game/Blueprints/Actors/BP_Hand.HighlightHand` _asbp_hand true)
  (set `self.EnableTrigger` true))

(event `self.HostButton.OnComponentEndOverlap`
  (params (OverlappedComponent :type "PrimitiveComponent Object Reference") (OtherActor :type "Actor Object Reference") (OtherComp :type "PrimitiveComponent Object Reference") (OtherBodyIndex :type Integer))
  ;[1 1 1] Revert Effect of Highlighted Controller
  (bind _asbp_hand (cast `/Game/Blueprints/Actors/BP_Hand` OtherActor))
  (`/Game/Blueprints/Actors/BP_Hand.HighlightHand` _asbp_hand false)
  (set `self.EnableTrigger` false :!label _label_2))

(event `self.JoinButton.OnComponentEndOverlap`
  (params (OverlappedComponent :type "PrimitiveComponent Object Reference") (OtherActor :type "Actor Object Reference") (OtherComp :type "PrimitiveComponent Object Reference") (OtherBodyIndex :type Integer))
  ;[1 1 1] Revert Effect of Highlighted Controller
  (bind _asbp_hand (cast `/Game/Blueprints/Actors/BP_Hand` OtherActor))
  (`/Game/Blueprints/Actors/BP_Hand.HighlightHand` _asbp_hand false)
  (goto _label_2))

(event `self.JoinButton.OnComponentBeginOverlap`
  (params (OverlappedComponent :type "PrimitiveComponent Object Reference") (OtherActor :type "Actor Object Reference") (OtherComp :type "PrimitiveComponent Object Reference") (OtherBodyIndex :type Integer) (bFromSweep :type Boolean) (SweepResult :type "HitResult Structure (by ref)"))
  ;[1 1 1] Highlight Controller on Overlap
  (bind _asbp_hand (cast `/Game/Blueprints/Actors/BP_Hand` OtherActor))
  (goto _label))

(fn `UserConstructionScript`)