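; BP_Activity is a named activity node actor that can be linked to other activities and highlighted by BP_Hand.
; Construction sets its label and color material, and Tick turns the label toward the player camera.
; ConnectActivity records new targets and spawns a BP_ConnectionPoint beam to each, returning true instead for duplicates or itself.
; Hand overlap toggles the Cube's visibility, and color functions apply dynamic material instances to ActivityBox.
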(event `self.ReceiveTick`
  (params (DeltaSeconds :type "Float (single-precision)"))
  (`SceneComponent.K2_SetWorldRotation` (`self.TextRender`) (`KismetMathLibrary.FindLookAtRotation` (`SceneComponent.K2_GetComponentLocation` (`self.TextRender`)) (`SceneComponent.K2_GetComponentLocation` (`PlayerCameraManager.TransformComponent` (`PlayerController.PlayerCameraManager` (`GameplayStatics.GetPlayerController` 0))))) false false))

(event `ShowConnection`
  (params (Target :type "Actor Object Reference"))
  (bind _returnvalue (`|SpawnActorFromClass` "/Game/Blueprints/ACtors/BP_ConnectionPoint_Auto9.BP_ConnectionPoint_C" (`self.GetTransform` Target) "Undefined" "OverrideRootScale" null (struct :`R` 0.653)))
  (`/Game/Blueprints/ACtors/BP_ConnectionPoint_Auto9.SetBeamSource` _returnvalue self)
  (`/Game/Blueprints/ACtors/BP_ConnectionPoint_Auto9.SetBeamTarget` _returnvalue Target))

(event `self.Cube.OnComponentBeginOverlap`
  (params (OverlappedComponent :type "PrimitiveComponent Object Reference") (OtherActor :type "Actor Object Reference") (OtherComp :type "PrimitiveComponent Object Reference") (OtherBodyIndex :type Integer) (bFromSweep :type Boolean) (SweepResult :type "HitResult Structure (by ref)"))
  (cast `/Game/Blueprints/Actors/BP_Hand` OtherActor)
  (`SceneComponent.SetVisibility` (`self.Cube`) true false))

(event `self.Cube.OnComponentEndOverlap`
  (params (OverlappedComponent :type "PrimitiveComponent Object Reference") (OtherActor :type "Actor Object Reference") (OtherComp :type "PrimitiveComponent Object Reference") (OtherBodyIndex :type Integer))
  (cast `/Game/Blueprints/Actors/BP_Hand` OtherActor)
  (`SceneComponent.SetVisibility` (`self.Cube`) false false))

(fn `ChangeActivityColor`
  (params (Color :type "LinearColor Structure"))
  (bind _returnvalue (`KismetMaterialLibrary.CreateDynamicMaterialInstance` "/Game/Models/ManMaterial.ManMaterial"))
  (`MaterialInstanceDynamic.SetVectorParameterValue` _returnvalue "ActivityColor" Color)
  (`PrimitiveComponent.SetMaterial` (`self.ActivityBox`) 0 _returnvalue))

(fn `ConnectActivity`
  (params (Target :type "/Game/Blueprints/ACtors/Activities/BP_Activity Object Reference"))
  (returns (AlreadyConnected :type Boolean))
  ;[1 1 1] Only connect if it is a new activity
  (if (not (`KismetArrayLibrary.Array_Contains` (`self.Targets`) Target))
    ;[1 1 1] Check if it is a activity to itself
    (if (== Target self)
      _
      (else
        ;[1 1 1] Create a visual connection between the two points
        (`KismetArrayLibrary.Array_Add` (`self.Targets`) Target)
        (`self.ShowConnection` Target)
        (return false))))
  (return true))

(fn `ResetActivityColor`
  (bind _returnvalue (`PrimitiveComponent.CreateDynamicMaterialInstance` (`self.ActivityBox`) 0 "/Game/Models/ManMaterial.ManMaterial"))
  (`MaterialInstanceDynamic.SetVectorParameterValue` _returnvalue "None" (`self.StandardColor`))
  (`PrimitiveComponent.SetMaterial` (`self.ActivityBox`) 0 _returnvalue))

(fn `UserConstructionScript`
  (`self.ResetActivityColor`)
  (`TextRenderComponent.K2_SetText` (`self.TextRender`) (`KismetTextLibrary.Conv_StringToText` (`self.ActivityName`))))