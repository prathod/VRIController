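; BP_Department is a placeable actor that acts as a portal, moving the multiplayer session to a department map.
; When a BP_PlayerPawn overlaps its Cube, the server runs a ServerTravel console command to the listen map matching the Level enum (BPMN, Finance or HR).
; The construction script writes the Level name into a TextRender label.
; BPMN Department leads to AdminMap, unlike the other two, whose map names match their departments.
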(event `self.Cube.OnComponentBeginOverlap`
  (params (OverlappedComponent :type "PrimitiveComponent Object Reference") (OtherActor :type "Actor Object Reference") (OtherComp :type "PrimitiveComponent Object Reference") (OtherBodyIndex :type Integer) (bFromSweep :type Boolean) (SweepResult :type "HitResult Structure (by ref)"))
  (`/Engine/EditorBlueprintResources/ActorMacros.Switch Has Authority`
    (:`Authority`
      (cast `/Game/Blueprints/Pawns/BP_PlayerPawn` OtherActor)
      (`self.TravelToDepartment`))))

(event `TravelToDepartment`
  (switch `/Game/Blueprints/Enum/Levels` (`self.Level`)
    (:`NewEnumerator0`
      (`KismetSystemLibrary.ExecuteConsoleCommand` "ServerTravel AdminMap?listen"))
    (:`NewEnumerator1`
      (`KismetSystemLibrary.ExecuteConsoleCommand` "ServerTravel FinanceMap?listen"))
    (:`NewEnumerator3`
      (`KismetSystemLibrary.ExecuteConsoleCommand` "ServerTravel HRMap?listen"))))

(fn `UserConstructionScript`
  (`TextRenderComponent.K2_SetText` (`self.TextRender`) (`KismetTextLibrary.Conv_StringToText` (`|GetEnumeratorNameAsString` (`self.Level`)))))