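; BP_Rol is a placeable role actor with a table, a stool and text labels that tints activities entering its area.
; The construction script writes the Rol value to five text components and applies a dynamic material tinted with RolColor to the table and stool.
; OverlapArea passes RolColor to any overlapping BP_Activity and resets that activity's color when the overlap ends.
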(event `self.OverlapArea.OnComponentBeginOverlap`
  (params (OverlappedComponent :type "PrimitiveComponent Object Reference") (OtherActor :type "Actor Object Reference") (OtherComp :type "PrimitiveComponent Object Reference") (OtherBodyIndex :type Integer) (bFromSweep :type Boolean) (SweepResult :type "HitResult Structure (by ref)"))
  (bind _asbp_activity (cast `/Game/Blueprints/ACtors/Activities/BP_Activity` OtherActor))
  (`/Game/Blueprints/ACtors/Activities/BP_Activity.ChangeActivityColor` _asbp_activity (`self.RolColor`)))

(event `self.OverlapArea.OnComponentEndOverlap`
  (params (OverlappedComponent :type "PrimitiveComponent Object Reference") (OtherActor :type "Actor Object Reference") (OtherComp :type "PrimitiveComponent Object Reference") (OtherBodyIndex :type Integer))
  (bind _asbp_activity (cast `/Game/Blueprints/ACtors/Activities/BP_Activity` OtherActor))
  (`/Game/Blueprints/ACtors/Activities/BP_Activity.ResetActivityColor` _asbp_activity))

(fn `UserConstructionScript`
  (`TextRenderComponent.K2_SetText` (`self.RolName4`) (`KismetTextLibrary.Conv_StringToText` (`self.Rol`)))
  (`TextRenderComponent.K2_SetText` (`self.RolName`) (`KismetTextLibrary.Conv_StringToText` (`self.Rol`)))
  (`TextRenderComponent.K2_SetText` (`self.RolName5`) (`KismetTextLibrary.Conv_StringToText` (`self.Rol`)))
  (`TextRenderComponent.K2_SetText` (`self.TextRender1`) (`KismetTextLibrary.Conv_StringToText` (`self.Rol`)))
  (`TextRenderComponent.K2_SetText` (`self.TextRender`) (`KismetTextLibrary.Conv_StringToText` (`self.Rol`)))
  (bind _returnvalue (`PrimitiveComponent.CreateDynamicMaterialInstance` (`self.simple_table`) 0 "/Game/Materials/RolMaterial.RolMaterial"))
  (`MaterialInstanceDynamic.SetVectorParameterValue` _returnvalue "RolColor" (`self.RolColor`))
  (`PrimitiveComponent.SetMaterial` (`self.simple_table`) 0 _returnvalue)
  (`PrimitiveComponent.SetMaterial` (`self.stul`) 0 _returnvalue))