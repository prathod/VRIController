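; BP_BPMWall is an actor that builds a wall of BPM lanes, one per BP_Rol role actor in the level.
; On BeginPlay it gathers all BP_Rol actors and passes them to CreateBPMLanes.
; That function spawns a BP_BPMLane for each role, starting at the wall's location and rotation, and attaches it to the wall.
; Each new lane's relative spawn point offsets the next, chaining the lanes in sequence.
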(event EventBeginPlay
  (bind _outactors (Actor|GetAllActorsOfClass "/Game/Blueprints/ACtors/BP_Rol.BP_Rol_C"))
  (bind _output_get (Variables|Default|SetRoles _outactors))
  (CallFunction|CreateBPMLanes _output_get))

(event Collision|EventActorBeginOverlap
  (params (OtherActor :type Actor%20Object%20Reference)))

(event EventTick
  (params (DeltaSeconds :type Float%20%28single-precision%29)))

(fn ConstructionScript)

(fn CreateBPMLanes
  (params (Roles :type Array%20of%20BP%20Rol%20Object%20References))
  (LocalVariables|SetNextSpawnTransform (Transformation|GetActorLocation))
  (for _array_element Roles
    (bind _returnvalue (Game|SpawnActorfromClass "/Game/Blueprints/ACtors/BP_BPMLane.BP_BPMLane_C" (Math|Transform|MakeTransform (LocalVariables|GetNextSpawnTransform) (Transformation|GetActorRotation)) "Undefined" 0 _array_element 0))
    (Transformation|AttachActorToActor _returnvalue self "None" "KeepWorld" "KeepWorld" "KeepWorld" true)
    (bind _getrelative (Default|GetRelativeSpawnPoint _returnvalue))
    (LocalVariables|SetNextSpawnTransform (+ _getrelative (LocalVariables|GetNextSpawnTransform)))))