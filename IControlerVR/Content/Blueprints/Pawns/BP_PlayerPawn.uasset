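; Multiplayer VR player pawn with motion-controller hands for drawing, moving activities, line-trace teleporting and toggling a toolbox.
; Trigger and grip input (O/P keys mirror grip) goes to BP_Hand child actors, with server-side ownership assignment for hands and toolbox.
; The local pawn reports head and hand transforms on a looping timer into SyncItems on the server.
; Non-local pawns interpolate toward those transforms each tick.
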(event Custom|ChangeOwnerOfHands
  (params (Playercontroller :type Player%20Controller%20Object%20Reference))
  ;[1 1 1] Give the client rights over the hand by setting the hand on the server
  (Networking|SwitchHasAuthority
    (:Authority
      (Actor|SetOwner (Variables|/Script/Engine.ChildActorComponent|GetChildActor (Variables|Default|GetRightHand)) Playercontroller)
      (Actor|SetOwner (Variables|/Script/Engine.ChildActorComponent|GetChildActor (Variables|Default|GetLeftHand)) Playercontroller)
      (Actor|SetOwner (Variables|/Script/Engine.ChildActorComponent|GetChildActor (Variables|Default|GetToolb)) Playercontroller))))

(event Custom|EnableDebugMode
  ;[1 1 1] Set the settings for the debug mode
  (Transformation|SetRelativeLocation (Variables|Default|GetHandHolderR) "80.000000,-50.000000, 0" false false)
  (Transformation|SetRelativeLocation (Variables|Default|GetHandHolderL) "80.000000,50.000000, 0" false false)
  (Class|HeadMountedDisplayFunctionLibrary|EnableHMD false)
  (Components|DestroyComponent (Variables|Default|GetCamera)))

(event EventBeginPlay
  (Class|HeadMountedDisplayFunctionLibrary|EnableHMD true)
  (bind _asbp_player_controller (Utilities|Casting|CastToBP_PlayerController (Game|GetPlayerController 0)))
  ;[1 1 1] Initializing
  (Variables|Default|SetBP_PlayerController _asbp_player_controller)
  (Utilities|FlowControl|Delay 1.0) ; Have to wait to know if the pawn is locally controlled
  (if (Pawn|IsLocallyControlled)
    (CallFunction|AddComponentforSyncing (Variables|Default|GetHandHolderR) 2.0)
    (CallFunction|AddComponentforSyncing (Variables|Default|GetHandHolderL) 2.0)
    (Utilities|Time|SetTimerbyFunctionName 0 "UpdateTransformToServer" (Variables|Settings|GetUpdateFrequency) true)
    (CallFunction|ChangeOwnerOfHands (Game|GetPlayerController 0))))

(event EventTick
  (params (DeltaSeconds :type Float%20%28single-precision%29))
  ;[1 1 1] Update the positions every tick
  (CallFunction|UpdateServerPositions))

(event Input|KeyboardEvents|MotionControllerLeftShoulder
  (params (Key :type Key%20Structure :default "AnyKey"))
  (bind _lefthand (Variables|Default|GetLeftHand))
  (bind _camera (Variables|Default|GetCamera))
  (bind _toolb (Variables|Default|GetToolb))
  (bind _returnvalue (Transformation|GetWorldTransform _lefthand))
  (bind _returnvalue_2 (Transformation|GetWorldLocation _camera))
  (bind _returnvalue_3 (Math|Vector|GetForwardVector _lefthand))
  (bind _returnvalue_4 (* _returnvalue_3 20))
  (bind _returnvalue_5 (+ (.location _returnvalue) _returnvalue_4))
  (bind _returnvalue_6 (Math|Rotator|FindLookatRotation _returnvalue_5 _returnvalue_2))
  ;[1 1 1] ToolBox spwan Activity
  (:Pressed
    (if (Rendering|IsVisible (Variables|Default|GetToolb))
      (Rendering|SetVisibility _toolb false true)
      (else
        (Rendering|SetVisibility _toolb true true)
        (Transformation|SetWorldLocationAndRotation (Variables|Default|GetToolb) _returnvalue_5 (Math|Rotator|MakeRotator 0.0 (.pitch _returnvalue_6) (.yaw _returnvalue_6)) false false)))))

(event Input|KeyboardEvents|MotionControllerRightTrigger
  (params (Key :type Key%20Structure :default "AnyKey"))
  (bind _righthand (Variables|Default|GetRightHand))
  (bind _childactor (Variables|/Script/Engine.ChildActorComponent|GetChildActor _righthand))
  ;[1 1 1] Start drawing with the right controller
  (:Pressed
    (if (Pawn|IsLocallyControlled)
      (bind _asbp_hand (Utilities|Casting|CastToBP_Hand _childactor))
      (Default|StartDrawingPatern _asbp_hand)
      (Variables|/Game/Blueprints/Actors/BP_Hand.BP_Hand_C|SetTriggerPressed _asbp_hand true)))
  (:Released
    (bind _asbp_hand_2 (Utilities|Casting|CastToBP_Hand _childactor))
    (Variables|/Game/Blueprints/Actors/BP_Hand.BP_Hand_C|SetTriggerPressed _asbp_hand_2 false)))

(event Input|KeyboardEvents|MotionControllerLeftThumbstick
  (params (Key :type Key%20Structure :default "AnyKey"))
  ;[1 1 1] Left Controller Teleportation
  (:Pressed
    (CallFunction|ChangeBeamVisibility (Variables|Default|GetTeleportBeamL) true))
  (:Released
    (bind _teleportlocation (CallFunction|GetTeleportLocation (Variables|Default|GetMotionControllerL)))
    (CallFunction|ChangeBeamVisibility (Variables|Default|GetTeleportBeamL) false)
    (if (Variables|Default|GetCanTeleport)
      (CallFunction|TeleporttoLocation _teleportlocation))))

(event Input|KeyboardEvents|MotionControllerRightThumbstick
  (params (Key :type Key%20Structure :default "AnyKey"))
  ;[1 1 1] Right Controller Teleportation
  (:Pressed
    (CallFunction|ChangeBeamVisibility (Variables|Default|GetTeleportBeamR) true))
  (:Released
    (bind _teleportlocation (CallFunction|GetTeleportLocation (Variables|Default|GetMotioncontrollerR)))
    (CallFunction|ChangeBeamVisibility (Variables|Default|GetTeleportBeamR) false)
    (if (Variables|Default|GetCanTeleport)
      (CallFunction|TeleporttoLocation _teleportlocation))))

(event Input|KeyboardEvents|MotionControllerRightGrip1
  (params (Key :type Key%20Structure :default "AnyKey"))
  ;[1 1 1] Grabbing with right motion controller
  (:Pressed
    (bind _ishand (CallFunction|HandCheck (Variables|Default|GetRightHand)))
    (Default|StartMovingActivity _ishand))
  (:Released
    (bind _ishand_2 (CallFunction|HandCheck (Variables|Default|GetRightHand)))
    (Default|StopMovingActivity _ishand_2)))

(event Input|KeyboardEvents|O
  (params (Key :type Key%20Structure :default "AnyKey"))
  ;[1 1 1] Grabbing with right motion controller
  (:Pressed
    (bind _ishand (CallFunction|HandCheck (Variables|Default|GetRightHand)))
    (Default|StartMovingActivity _ishand))
  (:Released
    (bind _ishand_2 (CallFunction|HandCheck (Variables|Default|GetRightHand)))
    (Default|StopMovingActivity _ishand_2)))

(event Input|KeyboardEvents|P
  (params (Key :type Key%20Structure :default "AnyKey"))
  ;[1 1 1] Grabbing with left motioncontroller
  (:Pressed
    (bind _ishand (CallFunction|HandCheck (Variables|Default|GetLeftHand)))
    (Default|StartMovingActivity _ishand))
  (:Released
    (bind _ishand_2 (CallFunction|HandCheck (Variables|Default|GetLeftHand)))
    (Default|StopMovingActivity _ishand_2)))

(event Input|KeyboardEvents|MotionControllerLeftGrip1
  (params (Key :type Key%20Structure :default "AnyKey"))
  ;[1 1 1] Grabbing with left motioncontroller
  (:Pressed
    (bind _ishand (CallFunction|HandCheck (Variables|Default|GetLeftHand)))
    (Default|StartMovingActivity _ishand))
  (:Released
    (bind _ishand_2 (CallFunction|HandCheck (Variables|Default|GetLeftHand)))
    (Default|StopMovingActivity _ishand_2)))

(event Input|KeyboardEvents|MotionControllerLeftTrigger
  (params (Key :type Key%20Structure :default "AnyKey"))
  (bind _lefthand (Variables|Default|GetLeftHand))
  (bind _childactor (Variables|/Script/Engine.ChildActorComponent|GetChildActor _lefthand))
  ;[1 1 1] Start drawing with the left controller
  (:Pressed
    (if (Pawn|IsLocallyControlled)
      (bind _asbp_hand (Utilities|Casting|CastToBP_Hand _childactor))
      (Default|StartDrawingPatern _asbp_hand)
      (Variables|/Game/Blueprints/Actors/BP_Hand.BP_Hand_C|SetTriggerPressed _asbp_hand true)))
  (:Released
    (bind _asbp_hand_2 (Utilities|Casting|CastToBP_Hand _childactor))
    (Variables|/Game/Blueprints/Actors/BP_Hand.BP_Hand_C|SetTriggerPressed _asbp_hand_2 false)))

(event Custom|UpdateServerPositions
  ;[1 1 1] Update the positions of the pawns of the other users
  (if (not (Pawn|IsLocallyControlled))
    (for _array_element (Variables|Default|GetSyncItems)
      (CallFunction|ChangeTransform _array_element))))

(event Custom|ServerUpdateTransform
  (params (New%20transform :type Sync%20Data%20Structure))
  ;[1 1 1] Set the transform on the server
  (Networking|SwitchHasAuthority
    (:Authority
      (bind (_contains _index) (CallFunction|ContainsSceneComponent (.SceneComponent (Utilities|Struct|BreakSyncData New%20transform))))
      (if _contains
        (Utilities|Array|SetArrayElem (Variables|Default|GetSyncItems) _index New%20transform)
        (else
          (Utilities|Array|Add (Variables|Default|GetSyncItems) New%20transform))))))

(event Custom|ChangeTransform
  (params (Syncdata :type Sync%20Data%20Structure))
  (bind _returnvalue (Transformation|GetWorldRotation (.scenecomponent Syncdata)))
  (bind _returnvalue_2 (Math|Rotator|Lerp(Rotator) (.worldrotation Syncdata) _returnvalue 0.1 true))
  ;[1 1 1] Change the current transform towards the server transform over time
  (Utilities|IsValid (.scenecomponent Syncdata)
    (:Is%20Valid
      (Transformation|SetWorldLocationAndRotation (.scenecomponent Syncdata) (Math|Interpolation|VInterpTo (Transformation|GetWorldLocation (.scenecomponent Syncdata)) (.worldlocation Syncdata) (Utilities|Time|GetWorldDeltaSeconds) (.syncspeed Syncdata)) (Math|Rotator|MakeRotator (.roll _returnvalue_2) (.pitch _returnvalue_2) (- (.yaw _returnvalue_2) 9e+01)) false false))))

(fn ConstructionScript)

(fn UpdateTransformtoServer
  (bind _returnvalue (Game|GetPlayerController 0))
  (bind _playercameramanager (Variables|/Script/Engine.PlayerController|GetPlayerCameraManager _returnvalue))
  (bind _transformcomponent (Variables|/Script/Engine.PlayerCameraManager|GetTransformComponent _playercameramanager))
  (if (Pawn|IsLocallyControlled)
    ;[1 1 1] Set the current transform towards the server
    (CallFunction|ServerUpdateTransform (Utilities|Struct|MakeSyncData (Variables|GetMeshComponent) (Transformation|GetWorldLocation _transformcomponent) (Transformation|GetWorldRotation _transformcomponent) 2.0))
    (for _array_element (Variables|Default|GetTransformComponents)
      (CallFunction|ServerUpdateTransform (Utilities|Struct|MakeSyncData (.scenecomponent _array_element) (Transformation|GetWorldLocation (.scenecomponent _array_element)) (Transformation|GetWorldRotation (.scenecomponent _array_element)) (.syncspeed _array_element))))))

(fn ContainsSceneComponent
  (params (SceneComponent :type Scene%20Component%20Object%20Reference))
  ;[1 1 1] Check if the array is already containing the item
  (for (_array_element _array_index) (Variables|Default|GetSyncItems)
    (if (== SceneComponent (.scenecomponent _array_element))
      (LocalVariables|SetContaining true)
      (LocalVariables|SetSyncDataIndex _array_index)))
  (return (LocalVariables|GetContaining) (LocalVariables|GetSyncDataIndex)))

(fn AddComponentforSyncing
  (params (New%20component :type Scene%20Component%20Object%20Reference) (Syncspeed :type Float%20%28single-precision%29))
  (if (Pawn|IsLocallyControlled)
    (Utilities|Array|Add (Variables|Default|GetTransformComponents) (Utilities|Struct|MakeSyncData New%20component (Transformation|GetWorldLocation New%20component) (Transformation|GetWorldRotation New%20component) Syncspeed))))

(fn HandCheck
  (params (Hand :type Child%20Actor%20Component%20Object%20Reference))
  (if (Pawn|IsLocallyControlled)
    (bind _asbp_hand (Utilities|Casting|CastToBP_Hand (Variables|/Script/Engine.ChildActorComponent|GetChildActor Hand)))
    (return _asbp_hand)))

(fn GetTeleportLocation
  (params (MotionController :type Scene%20Component%20Object%20Reference))
  (bind _returnvalue (Transformation|GetWorldLocation MotionController))
  (bind (_x _y) (Math|Vector|BreakVector _returnvalue))
  (bind _outhit (Collision|LineTraceByChannel _returnvalue (+ _returnvalue (* (Math|Vector|GetForwardVector MotionController) 1e+04)) "TraceTypeQuery1" false 0 "None"))
  (bind _asbp_activity (Utilities|Casting|CastToBP_Activity (.HitActor (Collision|BreakHitResult _outhit)))
    (:then
      (return (+ (/ (- (Math|Vector|MakeVector (.x (Transformation|GetActorLocation _asbp_activity)) (.y (Transformation|GetActorLocation _asbp_activity)) 0.0) (Math|Vector|MakeVector _x _y 0.0)) 2) (Math|Vector|MakeVector _x _y 0.0))))
    (:CastFailed
      (bind _output_get (Variables|Default|SetCanTeleport (> (Math|Vector|DotProduct (.Normal (Collision|BreakHitResult _outhit)) "0, 0,1.000000") 0.9)))
      (if _output_get
        (return (.Location (Collision|BreakHitResult _outhit)))
        (else
          (return "0, 0, 0"))))))

(fn TeleporttoLocation
  (params (Location :type Vector))
  (bind _camera (Variables|Default|GetCamera))
  (bind _relativelocation (Variables|/Script/Engine.SceneComponent|GetRelativeLocation _camera))
  (Transformation|SetActorLocationAndRotation (- Location (Math|Vector|MakeVector (.x _relativelocation) (.y _relativelocation) 0.0)) "0, 0, 0" false true))

(fn ChangeBeamVisibility
  (params (Beam :type Particle%20System%20Component%20Object%20Reference) (IsVisible :type Boolean))
  (Rendering|SetVisibility Beam IsVisible false))