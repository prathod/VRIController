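; Networked VR player pawn with two BP_Hand child actors for pattern drawing and grabbing, plus a left-shoulder toggle for spawning a toolbox.
; Trigger and grip inputs have keyboard equivalents and forward to the hands.
; The local pawn sends head and hand-holder transforms on a timer to the authority's SyncItems array, which non-local pawns interpolate toward each tick.
; Hand ownership is set under authority; the debug-mode setup is unwired.
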(event Custom|ChangeOwnerOfHands
  (params (Playercontroller :type Player%20Controller%20Object%20Reference))
  ;[1 1 1] Give the client rights over the hand by setting the hand on the server
  (Networking|SwitchHasAuthority
    (:Authority
      (Actor|SetOwner (Variables|/Script/Engine.ChildActorComponent|GetChildActor (Variables|Default|GetRightHand)) Playercontroller)
      (Actor|SetOwner (Variables|/Script/Engine.ChildActorComponent|GetChildActor (Variables|Default|GetLeftHand)) Playercontroller))))

(event Custom|EnableDebugMode
  ;[1 1 1] Set the settings for the debug mode
  (Transformation|SetRelativeLocation (Variables|Default|GetHandHolderR) "80.000000,-50.000000, 0" false false)
  (Transformation|SetRelativeLocation (Variables|Default|GetHandHolderL) "80.000000,50.000000, 0" false false)
  (Class|HeadMountedDisplayFunctionLibrary|EnableHMD false)
  (Components|DestroyComponent (Variables|Default|GetCamera)))

(event EventBeginPlay
  (bind _asbp_player_controller (Utilities|Casting|CastToBP_PlayerController (Game|GetPlayerController 0)))
  ;[1 1 1] Initializing
  (Variables|Default|SetBP_PlayerController _asbp_player_controller)
  (Utilities|FlowControl|Delay 1.0) ; Have to wait to know if the pawn is locally controlled
  (if (Pawn|IsLocallyControlled)
    (CallFunction|AddComponentforSyncing (Variables|Default|GetHandHolderR) 2.0)
    (CallFunction|AddComponentforSyncing (Variables|Default|GetHandHolderL) 2.0)
    (Utilities|Time|SetTimerbyFunctionName 0 "UpdateTransformToServer" (Variables|Settings|GetUpdateFrequency) true)
    (CallFunction|ChangeOwnerOfHands (Game|GetPlayerController 0))))

(event EventTick
  (params (DeltaSeconds :type Float%20%28single-precision%29))
  ;[1 1 1] Update the positions every tick
  (CallFunction|UpdateServerPositions))

(event Input|KeyboardEvents|K
  (params (Key :type Key%20Structure :default "AnyKey"))
  ;[1 1 1] Start drawing with the right controller
  (:Pressed
    (if (Pawn|IsLocallyControlled)
      (bind _asbp_hand (Utilities|Casting|CastToBP_Hand (Variables|/Script/Engine.ChildActorComponent|GetChildActor (Variables|Default|GetRightHand))))
      (Default|StartDrawingPatern _asbp_hand))))

(event Input|KeyboardEvents|MotionControllerRightTrigger
  (params (Key :type Key%20Structure :default "AnyKey"))
  ;[1 1 1] Start drawing with the right controller
  (:Pressed
    (if (Pawn|IsLocallyControlled)
      (bind _asbp_hand (Utilities|Casting|CastToBP_Hand (Variables|/Script/Engine.ChildActorComponent|GetChildActor (Variables|Default|GetRightHand))))
      (Default|StartDrawingPatern _asbp_hand))))

(event Input|KeyboardEvents|L
  (params (Key :type Key%20Structure :default "AnyKey"))
  ;[1 1 1] Start drawing with the left controller
  (:Pressed
    (if (Pawn|IsLocallyControlled)
      (bind _asbp_hand (Utilities|Casting|CastToBP_Hand (Variables|/Script/Engine.ChildActorComponent|GetChildActor (Variables|Default|GetLeftHand))))
      (Default|StartDrawingPatern _asbp_hand))))

(event Input|KeyboardEvents|MotionControllerLeftTrigger
  (params (Key :type Key%20Structure :default "AnyKey"))
  ;[1 1 1] Start drawing with the left controller
  (:Pressed
    (if (Pawn|IsLocallyControlled)
      (bind _asbp_hand (Utilities|Casting|CastToBP_Hand (Variables|/Script/Engine.ChildActorComponent|GetChildActor (Variables|Default|GetLeftHand))))
      (Default|StartDrawingPatern _asbp_hand))))

(event Input|KeyboardEvents|MotionControllerLeftShoulder
  (params (Key :type Key%20Structure :default "AnyKey"))
  (bind _lefthand (Variables|Default|GetLeftHand))
  (bind _returnvalue (Transformation|GetWorldTransform _lefthand))
  (:Pressed
    (Utilities|IsValid (Variables|Default|GettoolBox)
      (:Is%20Valid
        (Actor|DestroyActor (Variables|Default|GettoolBox)))
      (:Is%20Not%20Valid
        (bind _returnvalue_2 (Game|SpawnActorfromClass "/Game/Blueprints/ACtors/BP_Toolbox.BP_Toolbox_C" (Math|Transform|MakeTransform (+ (* (Math|Vector|GetForwardVector _lefthand) 20) (.location _returnvalue)) (Math|Rotator|MakeRotator (.roll (.rotation _returnvalue)) (+ (.pitch (.rotation _returnvalue)) -3e+01) (.yaw (.rotation _returnvalue))) "1,1,1") "Undefined" 0 0))
        (Variables|Default|SettoolBox _returnvalue_2)))))

(event Input|KeyboardEvents|MotionControllerRightGrip1
  (params (Key :type Key%20Structure :default "AnyKey"))
  ;[1 1 1] Grabbing with right motion controller
  (:Pressed
    (bind _ishand (CallFunction|HandCheck (Variables|Default|GetRightHand)))
    (Default|StartMovingActivity _ishand))
  (:Released
    (bind _ishand_2 (CallFunction|HandCheck (Variables|Default|GetRightHand)))
    (Default|StopMovingActivity _ishand_2)))

(event Input|KeyboardEvents|O
  (params (Key :type Key%20Structure :default "AnyKey"))
  ;[1 1 1] Grabbing with right motion controller
  (:Pressed
    (bind _ishand (CallFunction|HandCheck (Variables|Default|GetRightHand)))
    (Default|StartMovingActivity _ishand))
  (:Released
    (bind _ishand_2 (CallFunction|HandCheck (Variables|Default|GetRightHand)))
    (Default|StopMovingActivity _ishand_2)))

(event Input|KeyboardEvents|P
  (params (Key :type Key%20Structure :default "AnyKey"))
  ;[1 1 1] Grabbing with left motioncontroller
  (:Pressed
    (bind _ishand (CallFunction|HandCheck (Variables|Default|GetLeftHand)))
    (Default|StartMovingActivity _ishand))
  (:Released
    (bind _ishand_2 (CallFunction|HandCheck (Variables|Default|GetLeftHand)))
    (Default|StopMovingActivity _ishand_2)))

(event Input|KeyboardEvents|MotionControllerLeftGrip1
  (params (Key :type Key%20Structure :default "AnyKey"))
  ;[1 1 1] Grabbing with left motioncontroller
  (:Pressed
    (bind _ishand (CallFunction|HandCheck (Variables|Default|GetLeftHand)))
    (Default|StartMovingActivity _ishand))
  (:Released
    (bind _ishand_2 (CallFunction|HandCheck (Variables|Default|GetLeftHand)))
    (Default|StopMovingActivity _ishand_2)))

(event Custom|UpdateServerPositions
  ;[1 1 1] Update the positions of the pawns of the other users
  (if (not (Pawn|IsLocallyControlled))
    (for _array_element (Variables|Default|GetSyncItems)
      (CallFunction|ChangeTransform _array_element))))

(event Custom|ServerUpdateTransform
  (params (New%20transform :type Sync%20Data%20Structure))
  ;[1 1 1] Set the transform on the server
  (Networking|SwitchHasAuthority
    (:Authority
      (bind (_contains _index) (CallFunction|ContainsSceneComponent (.SceneComponent (Utilities|Struct|BreakSyncData New%20transform))))
      (if _contains
        (Utilities|Array|SetArrayElem (Variables|Default|GetSyncItems) _index New%20transform)
        (else
          (Utilities|Array|Add (Variables|Default|GetSyncItems) New%20transform))))))

(event Custom|ChangeTransform
  (params (Syncdata :type Sync%20Data%20Structure))
  ;[1 1 1] Change the current transform towards the server transform over time
  (Utilities|IsValid (.scenecomponent Syncdata)
    (:Is%20Valid
      (Transformation|SetWorldLocationAndRotation (.scenecomponent Syncdata) (Math|Interpolation|VInterpTo (Transformation|GetWorldLocation (.scenecomponent Syncdata)) (.worldlocation Syncdata) (Utilities|Time|GetWorldDeltaSeconds) (.syncspeed Syncdata)) (Math|Rotator|Lerp(Rotator) (.worldrotation Syncdata) (Transformation|GetWorldRotation (.scenecomponent Syncdata)) 0.1 true) false false))))

(fn ConstructionScript)

(fn UpdateTransformtoServer
  (bind _returnvalue (Game|GetPlayerController 0))
  (bind _playercameramanager (Variables|/Script/Engine.PlayerController|GetPlayerCameraManager _returnvalue))
  (bind _transformcomponent (Variables|/Script/Engine.PlayerCameraManager|GetTransformComponent _playercameramanager))
  (bind _returnvalue_2 (Transformation|GetWorldRotation _transformcomponent))
  (if (Pawn|IsLocallyControlled)
    ;[1 1 1] Set the current transform towards the server
    (CallFunction|ServerUpdateTransform (Utilities|Struct|MakeSyncData (Variables|GetMeshComponent) (Transformation|GetWorldLocation _transformcomponent) (Math|Rotator|MakeRotator (- (.roll _returnvalue_2) 9e+01) (.pitch _returnvalue_2) (- (.yaw _returnvalue_2) 9e+01)) 2.0))
    (for _array_element (Variables|Default|GetTransformComponents)
      (CallFunction|ServerUpdateTransform (Utilities|Struct|MakeSyncData (.scenecomponent _array_element) (Transformation|GetWorldLocation (.scenecomponent _array_element)) (Transformation|GetWorldRotation (.scenecomponent _array_element)) (.syncspeed _array_element))))))

(fn ContainsSceneComponent
  (params (SceneComponent :type Scene%20Component%20Object%20Reference))
  ;[1 1 1] Check if the array is already containing the item
  (for (_array_element _array_index) (Variables|Default|GetSyncItems)
    (if (== SceneComponent (.scenecomponent _array_element))
      (LocalVariables|SetContaining true)
      (LocalVariables|SetSyncDataIndex _array_index)))
  (return (LocalVariables|GetContaining) (LocalVariables|GetSyncDataIndex)))

(fn AddComponentforSyncing
  (params (New%20component :type Scene%20Component%20Object%20Reference) (Syncspeed :type Float%20%28single-precision%29))
  (if (Pawn|IsLocallyControlled)
    (Utilities|Array|Add (Variables|Default|GetTransformComponents) (Utilities|Struct|MakeSyncData New%20component (Transformation|GetWorldLocation New%20component) (Transformation|GetWorldRotation New%20component) Syncspeed))))

(fn HandCheck
  (params (Hand :type Child%20Actor%20Component%20Object%20Reference))
  (if (Pawn|IsLocallyControlled)
    (bind _asbp_hand (Utilities|Casting|CastToBP_Hand (Variables|/Script/Engine.ChildActorComponent|GetChildActor Hand)))
    (return _asbp_hand)))